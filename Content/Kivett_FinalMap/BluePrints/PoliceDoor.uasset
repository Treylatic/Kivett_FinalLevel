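; PoliceDoor is a door Blueprint that swings open once the player has collected every clue.
; Each Tick it compares the FirstPersonCharacter's Clues with TotalClues and plays a timeline when the total is reached.
; The timeline lerps the Door's relative rotation from its starting value to an absolute 90-degree yaw, keeping roll and pitch.
; Activating the Door component also enables player input on the actor, though no input events are defined.
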(event OnComponentActivated(Door)
  (params (Component :type Actor%20Component%20Object%20Reference) (bReset :type Boolean))
  (Input|EnableInput (Game|GetPlayerController 0)))

(event EventBeginPlay
  (bind _door (Variables|Default|GetDoor))
  (bind _relativerotation (Variables|/Script/Engine.SceneComponent|GetRelativeRotation _door))
  (bind (_roll _pitch) (Math|Rotator|BreakRotator _relativerotation))
  (Variables|Default|SetRotateBegin _relativerotation)
  (Variables|Default|SetRotateEnd (Math|Rotator|MakeRotator _roll _pitch 9e+01)))

(event EventTick
  (params (DeltaSeconds :type Float%20%28single-precision%29))
  (bind _asfirst_person_character (Utilities|Casting|CastToFirstPersonCharacter (Game|Player|GetPlayerPawn 0)))
  (if (>= (Variables|/Game/FirstPersonBP/Blueprints/FirstPersonCharacter.FirstPersonCharacter_C|GetClues _asfirst_person_character) (Variables|/Game/FirstPersonBP/Blueprints/FirstPersonCharacter.FirstPersonCharacter_C|GetTotalClues _asfirst_person_character))
    (bind _door_open (Timeline|Timeline_0 Play)
      (:Update
        (Transformation|SetRelativeRotation (Variables|Default|GetDoor) (Math|Rotator|Lerp(Rotator) (Variables|Default|GetRotateBegin) (Variables|Default|GetRotateEnd) _door_open) false false)))))

(fn ConstructionScript)