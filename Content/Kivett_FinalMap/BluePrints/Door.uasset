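; A door actor that swings open when something overlaps its Trigger and closes when the overlap ends.
; BeginPlay stores the Door component's relative rotation as the start and builds an end rotation with yaw set to an absolute 90 degrees.
; A timeline plays or reverses on overlap, lerping between the two rotations.
; Activating the Door component also enables input for player 0, though no input events are defined.
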(event OnComponentBeginOverlap(Trigger)
  (params (OverlappedComponent :type Primitive%20Component%20Object%20Reference) (OtherActor :type Actor%20Object%20Reference) (OtherComp :type Primitive%20Component%20Object%20Reference) (OtherBodyIndex :type Integer) (bFromSweep :type Boolean) (SweepResult :type Hit%20Result%20Structure%20%28by%20ref%29))
  (bind _door_open (Timeline|Timeline_0 Play)
    (:Update
      (Transformation|SetRelativeRotation (Variables|Default|GetDoor) (Math|Rotator|Lerp(Rotator) (Variables|Default|GetRotateBegin) (Variables|Default|GetRotateEnd) _door_open) false false))))

(event OnComponentActivated(Door)
  (params (Component :type Actor%20Component%20Object%20Reference) (bReset :type Boolean))
  (Input|EnableInput (Game|GetPlayerController 0)))

(event OnComponentEndOverlap(Trigger)
  (params (OverlappedComponent :type Primitive%20Component%20Object%20Reference) (OtherActor :type Actor%20Object%20Reference) (OtherComp :type Primitive%20Component%20Object%20Reference) (OtherBodyIndex :type Integer))
  (bind _door_open (Timeline|Timeline_0 Reverse)
    (:Update
      (Transformation|SetRelativeRotation (Variables|Default|GetDoor) (Math|Rotator|Lerp(Rotator) (Variables|Default|GetRotateBegin) (Variables|Default|GetRotateEnd) _door_open) false false))))

(event EventBeginPlay
  (bind _door (Variables|Default|GetDoor))
  (bind _relativerotation (Variables|/Script/Engine.SceneComponent|GetRelativeRotation _door))
  (bind (_roll _pitch) (Math|Rotator|BreakRotator _relativerotation))
  (Variables|Default|SetRotateBegin _relativerotation)
  (Variables|Default|SetRotateEnd (Math|Rotator|MakeRotator _roll _pitch 9e+01)))

(fn ConstructionScript)